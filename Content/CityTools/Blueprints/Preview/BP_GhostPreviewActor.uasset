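; BP_GhostPreviewActor is a preview actor in the city tools that positions a ghost mesh at a given world location.
; UpdatePreviewLocation moves PreviewMesh to that location without sweeping or teleporting.
; When SnapToGrid is on, it snaps X and Y to GridSize and keeps Z unchanged.
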(fn ConstructionScript)

(fn UpdatePreviewLocation
  (params (WorldLocation :type Vector))
  (if (Variables|Default|GetbSnapToGrid)
    (Transformation|SetWorldLocation (Variables|Default|GetPreviewMesh) (Math|Vector|MakeVector (Math|Float|SnapToGrid(Float) (.x WorldLocation) (Variables|Default|GetGridSize)) (Math|Float|SnapToGrid(Float) (.y WorldLocation) (Variables|Default|GetGridSize)) (.z WorldLocation)) false false)
    (else
      (Transformation|SetWorldLocation (Variables|Default|GetPreviewMesh) (Math|Vector|MakeVector (.x WorldLocation) (.y WorldLocation) (.z WorldLocation)) false false))))