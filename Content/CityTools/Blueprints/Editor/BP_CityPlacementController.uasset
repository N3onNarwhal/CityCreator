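; Editor-side controller for city building placement that spawns static mesh actors from a BuildingSet.
; OnEditorPlacement checks that the set is valid, then spawns a StaticMeshActor at the given world position using the current option's mesh, rotation and scale.
; NextBuilding and PrevBuilding step the current index, clamped to the list bounds without wrapping.
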(event EventBeginPlay)

(event Collision|EventActorBeginOverlap
  (params (OtherActor :type Actor%20Object%20Reference)))

(event EventTick
  (params (DeltaSeconds :type Float%20%28single-precision%29)))

(event EventOnEditorPlacement
  (params (WorldPosition :type Vector :default "0, 0, 0"))
  (bind _buildingset (Variables|Default|GetBuildingSet))
  (Utilities|IsValid _buildingset
    (:Is%20Valid
      (Variables|Default|SetBuildingOption (Utilities|Array|Get(acopy) (Variables|/Game/CityTools/Blueprints/Data/PDA_BuildingSet.PDA_BuildingSet_C|GetBuildings _buildingset) (Variables|Default|GetCurrentBuildingIndex)))
      (bind _returnvalue (Game|SpawnActorfromClass "/Script/Engine.StaticMeshActor" (Math|Transform|MakeTransform WorldPosition (.Rotation (Utilities|Struct|BreakST_BuildingOption (Variables|Default|GetBuildingOption))) (.Scale (Utilities|Struct|BreakST_BuildingOption (Variables|Default|GetBuildingOption)))) "Undefined" "MultiplyWithRoot" 0 0))
      (Components|StaticMesh|SetStaticMesh (Variables|/Script/Engine.StaticMeshActor|GetStaticMeshComponent _returnvalue) (.Mesh (Utilities|Struct|BreakST_BuildingOption (Variables|Default|GetBuildingOption)))))))

(fn ConstructionScript)

(fn NextBuilding
  (bind _result (Math|Integer|IncrementInt (Variables|Default|GetCurrentBuildingIndex))
    (:%20%20
      (Variables|Default|SetCurrentBuildingIndex (Math|Integer|Clamp(Integer) _result 0 (- (Utilities|Array|Length (Variables|/Game/CityTools/Blueprints/Data/PDA_BuildingSet.PDA_BuildingSet_C|GetBuildings (Variables|Default|GetBuildingSet))) 1))))))

(fn PrevBuilding
  (bind _result (Math|Integer|DecrementInt (Variables|Default|GetCurrentBuildingIndex))
    (:%20%20
      (Variables|Default|SetCurrentBuildingIndex (Math|Integer|Clamp(Integer) _result 0 (- (Utilities|Array|Length (Variables|/Game/CityTools/Blueprints/Data/PDA_BuildingSet.PDA_BuildingSet_C|GetBuildings (Variables|Default|GetBuildingSet))) 1))))))