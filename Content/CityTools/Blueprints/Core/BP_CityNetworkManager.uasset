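; BP_CityNetworkManager stores the city's road network for the city tools as arrays of road segment and node structs.
; AddRoad and AddNode append entries with incrementing IDs, and new roads get a fixed default width and lane count.
; It also clears the network and resets its counters, exposes both arrays through getters, and stores the current placement mode.
; It only holds data, with no mesh spawning or linking of roads to nodes.
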(event EventBeginPlay
  (Development|PrintString "City Manager Ready"))

(fn ConstructionScript)

(fn AddRoad
  (params (Start :type Vector) (End :type Vector))
  (Utilities|Array|Add (Variables|Default|GetRoads) (Utilities|Struct|MakeST_RoadSegment (Variables|Default|GetNextRoadID) Start End 4e+02 2))
  (Math|Integer|IncrementInt (Variables|Default|GetNextRoadID)
    (:%20%20
      (Development|PrintString "Added road"))))

(fn AddNode
  (params (Position :type Vector))
  (Utilities|Array|Add (Variables|Default|GetNodes) (Utilities|Struct|MakeST_Node (Variables|Default|GetNextNodeID) Position))
  (Math|Integer|IncrementInt (Variables|Default|GetNextNodeID)
    (:%20%20
      (Development|PrintString "Node added"))))

(fn ClearNetwork
  (Utilities|Array|Clear (Variables|Default|GetRoads))
  (Utilities|Array|Clear (Variables|Default|GetNodes))
  (Variables|Default|SetNextRoadID 0)
  (Variables|Default|SetNextNodeID 0))

(fn SetPlacementMode
  (params (NewMode :type EN_PlacementMode%20Enum :default "NewEnumerator0"))
  (Variables|Default|SetCurrentMode NewMode))

(fn GetRoads
  (return (Variables|Default|GetRoads)))

(fn GetNodes
  (return (Variables|Default|GetNodes)))