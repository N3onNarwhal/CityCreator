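; BP_CityDebugVisualizer is a city tools Blueprint that, despite its visualizer name, only records road and node counts from the city network and draws nothing.
; BeginPlay caches the first BP_CityNetworkManager found in the level as ManagerRef.
; Refresh, which nothing in this Blueprint calls, copies the lengths of that manager's Roads and Nodes arrays into NumRoads and NumNodes when the reference is valid.
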(event EventBeginPlay
  (bind _outactors (Actor|GetAllActorsOfClass "/Game/CityTools/Blueprints/Core/BP_CityNetworkManager.BP_CityNetworkManager_C"))
  (Variables|Default|SetManagerRef (Utilities|Array|Get(acopy) _outactors)))

(fn ConstructionScript)

(fn Refresh
  (Utilities|IsValid (Variables|Default|GetManagerRef)
    (:Is%20Valid
      (Variables|Default|SetNumRoads (Utilities|Array|Length (Variables|/Game/CityTools/Blueprints/Core/BP_CityNetworkManager.BP_CityNetworkManager_C|GetRoads (Variables|Default|GetManagerRef))))
      (Variables|Default|SetNumNodes (Utilities|Array|Length (Variables|/Game/CityTools/Blueprints/Core/BP_CityNetworkManager.BP_CityNetworkManager_C|GetNodes (Variables|Default|GetManagerRef)))))
    (:Is%20Not%20Valid
      (return))))